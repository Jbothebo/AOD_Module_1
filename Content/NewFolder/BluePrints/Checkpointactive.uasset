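; Checkpoint logic that stores a respawn-style transform in the Char_Male character's CheckPoint variable.
; ActivateCheckPoint casts the passed actor to Char_Male, saves its own owner's location as a location-only transform, and prints the result for debugging.
; SetCheckPoint is a separate function that instead saves the player pawn's current full transform, with its debug print left unconnected.
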(event Custom|Activate%20Check%20Point
  (params (OtherActor :type Actor%20Object%20Reference))
  (bind _aschar_male (Utilities|Casting|CastToChar_Male OtherActor))
  (bind _output_get (Variables|/Game/BluePrints/Char_Male.Char_Male_C|SetCheckPoint _aschar_male (Math|Conversions|ToTransform(Vector) (Transformation|GetActorLocation (Components|GetOwner)))))
  (Development|PrintString (Utilities|String|ToString(Transform) _output_get)))

(fn SetCheckPoint
  (bind _aschar_male (Utilities|Casting|CastToChar_Male (Game|Player|GetPlayerPawn 0)))
  (bind _output_get (Variables|/Game/BluePrints/Char_Male.Char_Male_C|SetCheckPoint _aschar_male (Transformation|GetActorTransform _aschar_male))))