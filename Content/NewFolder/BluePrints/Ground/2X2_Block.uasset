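; 2X2 ground block that behaves as a one-way platform, solid only while the player is above it.
; Each Tick it compares player 0's Z, less a hardcoded offset, with its own Z and toggles RenderComponent between QueryAndPhysics and NoCollision.
; The construction script starts it with no collision and can print the block's Z when the NewVar0 flag is set.
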(event EventTick
  (params (DeltaSeconds :type Float%20%28single-precision%29))
  (if (> (- (.Z (Math|Vector|BreakVector (Transformation|GetActorLocation (Game|GetPlayerCharacter 0)))) (+ 5e+01 84.0)) (.Z (Math|Vector|BreakVector (Transformation|GetActorLocation))))
    (Collision|SetCollisionEnabled (Variables|Default|GetRenderComponent) "QueryAndPhysics")
    (else
      (Collision|SetCollisionEnabled (Variables|Default|GetRenderComponent) "NoCollision"))))

(fn ConstructionScript
  (Collision|SetCollisionEnabled (Variables|Default|GetRenderComponent) "NoCollision")
  (if (Variables|Default|GetNewVar_0)
    (Development|PrintString (Utilities|String|ToString(Float) (.Z (Math|Vector|BreakVector (Transformation|GetActorLocation)))))))