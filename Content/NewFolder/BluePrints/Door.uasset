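; Interactable 2D door Blueprint that transitions the player to a connecting level.
; A box trigger enables input and shows a text prompt while overlapped, then disables both on exit.
; Pressing F alternates via FlipFlop: the first press swaps the sprite, fades the camera and loads ConnectingLevel after a short delay, while the next press swaps to the other sprite.
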(event OnComponentBeginOverlap(Box)
  (params (OverlappedComponent :type Primitive%20Component%20Object%20Reference) (OtherActor :type Actor%20Object%20Reference) (OtherComp :type Primitive%20Component%20Object%20Reference) (OtherBodyIndex :type Integer) (bFromSweep :type Boolean) (SweepResult :type Hit%20Result%20Structure%20%28by%20ref%29))
  (Input|EnableInput (Game|GetPlayerController 0))
  (Rendering|SetVisibility (Variables|Default|GetTextRender) true false))

(event OnComponentEndOverlap(Box)
  (params (OverlappedComponent :type Primitive%20Component%20Object%20Reference) (OtherActor :type Actor%20Object%20Reference) (OtherComp :type Primitive%20Component%20Object%20Reference) (OtherBodyIndex :type Integer))
  (Input|DisableInput (Game|GetPlayerController 0))
  (Rendering|SetVisibility (Variables|Default|GetTextRender) false false))

(event Input|KeyboardEvents|F
  (params (Key :type Key%20Structure))
  (:Pressed
    (Utilities|FlowControl|FlipFlop
      (:A
        (Rendering|Components|Sprite|SetSprite (Variables|Default|GetPaperSprite) "/Game/Sprites/ground_textures_Sprite_9.ground_textures_Sprite_9")
        (CameraFades|StartCameraFade :self (Game|GetPlayerCameraManager 0) :ToAlpha 2.0 :Duration 1.5)
        (Utilities|FlowControl|Delay 1.0)
        (Game|OpenLevel(byName) (Variables|Default|GetConnecting%20Level)))
      (:B
        (Rendering|Components|Sprite|SetSprite (Variables|Default|GetPaperSprite) "/Game/Sprites/ground_textures_Sprite_8.ground_textures_Sprite_8")))))

(fn ConstructionScript)