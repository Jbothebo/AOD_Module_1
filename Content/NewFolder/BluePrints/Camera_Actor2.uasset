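; Camera actor that follows player 0's character, with its height influenced by a LowerBound value.
; Each Tick checks the player's Z against a fixed threshold, reversing a timeline at or below it and playing it forward above.
; Timeline updates sweep the actor to the player's X and Y, lerping Z between the player's height and LowerBound by the track value.
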(event EventTick
  (params (DeltaSeconds :type Float%20%28single-precision%29))
  (bind _returnvalue (Game|GetPlayerCharacter 0))
  (bind _returnvalue_2 (Game|GetPlayerCharacter 0))
  (bind _returnvalue_3 (Transformation|GetActorLocation _returnvalue_2))
  (bind _returnvalue_4 (Transformation|GetActorLocation _returnvalue))
  (bind (_x _y _z) (Math|Vector|BreakVector _returnvalue_3))
  (bind (_x_2 _y_2) (Math|Vector|BreakVector _returnvalue_4))
  (if (<= _z 342.0)
    (bind _newtrack_0 (Timeline|Timeline_0 Reverse)
      (:Update
        (Transformation|SetActorLocation (Math|Vector|MakeVector _x_2 _y_2 (Math|Float|Lerp _z (Variables|Default|GetLower%20bound) _newtrack_0)) true false)))
    (else
      (Timeline|Timeline_0 Play))))

(fn ConstructionScript)