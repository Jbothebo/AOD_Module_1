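; NPC actor that shows a short dialogue in a text render and can optionally end the game.
; Box overlap toggles text visibility and player input; leaving also resets the dialogue to the secondary prompt.
; Pressing R steps through three lines via a selection counter, then clears the text and, if EndGame is set, quits after a delay.
; Tick refreshes the text and flips the actor according to the player's side on X.
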(event OnComponentBeginOverlap(Box)
  (params (OverlappedComponent :type Primitive%20Component%20Object%20Reference) (OtherActor :type Actor%20Object%20Reference) (OtherComp :type Primitive%20Component%20Object%20Reference) (OtherBodyIndex :type Integer) (bFromSweep :type Boolean) (SweepResult :type Hit%20Result%20Structure%20%28by%20ref%29))
  (Input|EnableInput (Game|GetPlayerController 0))
  (Rendering|ToggleVisibility (Variables|Default|GetTextRender) false))

(event OnComponentEndOverlap(Box)
  (params (OverlappedComponent :type Primitive%20Component%20Object%20Reference) (OtherActor :type Actor%20Object%20Reference) (OtherComp :type Primitive%20Component%20Object%20Reference) (OtherBodyIndex :type Integer))
  (Variables|Default|SetPropmt%20text (Variables|Default|GetSecondary%20Prompt))
  (Variables|Default|SetSelcetion 0)
  (Input|DisableInput (Game|GetPlayerController 0))
  (Rendering|ToggleVisibility (Variables|Default|GetTextRender) false))

(event Custom|Set%20Text
  (bind _output_get (Variables|Default|SetPropmt%20text (Variables|Default|GetPropmt%20text)))
  (Rendering|Components|TextRender|SetText (Variables|Default|GetTextRender) _output_get))

(event Custom|Rotation
  (params (DeltaSeconds :type Float%20%28single-precision%29))
  (if (< (.X (Math|Vector|BreakVector (Transformation|GetActorLocation (Game|GetPlayerCharacter 0)))) (.X (Math|Vector|BreakVector (Transformation|GetActorLocation))))
    (Transformation|SetActorRotation "0,180.000000, 0")
    (else
      (Transformation|SetActorRotation "0,0.000000, 0"))))

(event EventTick
  (params (DeltaSeconds :type Float%20%28single-precision%29))
  (CallFunction|Rotation 0.0)
  (CallFunction|SetText))

(event Input|KeyboardEvents|R
  (params (Key :type Key%20Structure))
  (:Pressed
    (if (== (Variables|Default|GetSelcetion) 0)
      (Variables|Default|SetPropmt%20text (Variables|Default|GetNewVar_0))
      (Variables|Default|SetSelcetion 1)
      (elif (== (Variables|Default|GetSelcetion) 1)
        (Variables|Default|SetPropmt%20text (Variables|Default|GetNewVar_1))
        (Variables|Default|SetSelcetion 2)
        (elif (== (Variables|Default|GetSelcetion) 2)
          (Variables|Default|SetPropmt%20text (Variables|Default|GetNewVar_2))
          (Variables|Default|SetSelcetion 3)
          (else
            (Variables|Default|SetPropmt%20text "")
            (if (Variables|Default|GetEnd%20Game?)
              (Utilities|FlowControl|Delay 2.0)
              (Game|QuitGame 0 "Quit"))))))))

(fn ConstructionScript)