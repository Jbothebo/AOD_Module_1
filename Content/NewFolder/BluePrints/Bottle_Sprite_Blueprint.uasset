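; Bottle pickup actor that bobs in place and marks the player's game state as holding an item when overlapped.
; A self-retriggering Hover event alternates a timeline forward and in reverse through a FlipFlop, lerping Z 10 units below its starting height and back.
; On any actor overlap, it sets HasItem on the Global_Var game instance and destroys itself.
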(event Custom|Hover
  (bind _returnvalue (Transformation|GetActorLocation))
  (bind _position (Variables|Default|GetPosition))
  (bind (_x _y) (Math|Vector|BreakVector _returnvalue))
  (Utilities|FlowControl|FlipFlop
    (:A
      (bind _newtrack_0 (Timeline|Timeline_0 PlayFromStart)
        (:Update
          (Transformation|SetActorLocation (Math|Vector|MakeVector _x _y (Math|Float|Lerp _position (- _position 1e+01) _newtrack_0)) false false))
        (:Finished
          (CallFunction|Hover))))
    (:B
      (Timeline|Timeline_0 ReverseFromEnd))))

(event Collision|EventActorBeginOverlap
  (params (OtherActor :type Actor%20Object%20Reference))
  (bind _asglobal_var (Utilities|Casting|CastToGlobal_Var (Game|GetGameInstance)))
  (Variables|/Game/BluePrints/Global_Var.Global_Var_C|SetHas%20Item _asglobal_var true)
  (Actor|DestroyActor))

(event EventBeginPlay
  (Variables|Default|SetPosition (.Z (Math|Vector|BreakVector (Transformation|GetActorLocation))))
  (CallFunction|Hover))

(fn ConstructionScript)