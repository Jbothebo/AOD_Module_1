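; Paper2D platform actor that can move back and forth along X, Z or both, depending on its CanMoveX and CanMoveZ flags.
; Shortly after BeginPlay, each enabled axis runs a timeline lerp from start position to target, using FlipFlop on completion to ping-pong.
; On any actor overlap, it disables sprite collision if the player's X velocity is positive (commented as vertical), otherwise enables it.
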(event Custom|Move%20Z
  (bind _returnvalue (Transformation|GetActorLocation))
  (bind (_x _y) (Math|Vector|BreakVector _returnvalue))
  (Utilities|FlowControl|FlipFlop
    (:A
      (bind _newtrack_0 (Timeline|Timeline_1 PlayFromStart)
        (:Update
          (Transformation|SetActorLocation (Math|Vector|MakeVector _x _y (Math|Float|Lerp (Variables|Default|GetPosition%20Z) (Variables|Default|GetMove%20to%20Z) _newtrack_0)) false false))
        (:Finished
          (CallFunction|MoveZ))))
    (:B
      (Timeline|Timeline_1 ReverseFromEnd))))

(event Custom|Move%20X
  (bind _returnvalue (Transformation|GetActorLocation))
  (bind (_x _y _z) (Math|Vector|BreakVector _returnvalue))
  (Utilities|FlowControl|FlipFlop
    (:A
      (bind _newtrack_0 (Timeline|Timeline_0 PlayFromStart)
        (:Update
          (Transformation|SetActorLocation (Math|Vector|MakeVector (Math|Float|Lerp (Variables|Default|GetPosition%20X) (Variables|Default|GetMove%20to%20X) _newtrack_0) _y _z) false false))
        (:Finished
          (CallFunction|MoveX))))
    (:B
      (Timeline|Timeline_0 ReverseFromEnd))))

(event Custom|Hover
  (if (Variables|Default|GetCan%20move%20X)
    (CallFunction|MoveX))
  (if (Variables|Default|GetCan%20Move%20Z)
    (CallFunction|MoveZ)))

(event EventBeginPlay
  (bind _returnvalue (Transformation|GetActorLocation))
  (bind (_x _y _z) (Math|Vector|BreakVector _returnvalue))
  (Variables|Default|SetPosition%20X _x)
  (Variables|Default|SetPosition%20Z _z)
  (Utilities|FlowControl|Delay 0.2)
  (CallFunction|Hover))

(event Collision|EventActorBeginOverlap
  (params (OtherActor :type Actor%20Object%20Reference))
  (bind _papersprite (Variables|Default|GetPaperSprite))
  ;[1 1 1] Checks if player will interact with platform
  (bind _output_get (Variables|Default|SetIs%20in%20Area true))
  (if _output_get
    ;[1 1 1] Turns on collision based on player vertical velocity
    (if (> (.X (Math|Vector|BreakVector (Transformation|GetVelocity (Game|GetPlayerCharacter 0)))) 0.0)
      (Collision|SetCollisionEnabled _papersprite "NoCollision")
      (else
        (Collision|SetCollisionEnabled _papersprite "QueryAndPhysics")))))

(fn ConstructionScript)