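; Player character for a 2D side-scroller, with variable-height jumping, flipbook animation and checkpoint respawn.
; Horizontal input moves and flips the character, then feeds movement and death flags into a state function selecting Idle, Run, Fall or Dead.
; Tick offsets the camera boom to hold height above a threshold and triggers death below kill height: fade, destroy, respawn at construction-time transform.
; It also creates the HUD and handles pause and debug keys.
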(event Custom|Update%20Anim
  ;[1 1 1] Collect movement data
  (Variables|Default|SetIs%20Moving (> (Math|Vector|VectorLength (Transformation|GetVelocity)) 0.0))
  (Variables|Default|SetIs%20Falling (AI|Components|NavMovement|IsFalling (Variables|Character|GetCharacterMovement)))
  ;[1 1 1] Get and Set Animation
  (bind _flip_book (Animations|AnimationStateMachine (Variables|Default|GetIs%20Falling) (Variables|Default|GetIs%20Moving) (Variables|Default|GetIs%20Dead)))
  (Sprite|SetFlipbook (Variables|Default|GetSprite) _flip_book))

(event Custom|Set%20Hud
  ;[1 1 1] Set Hud
  (Utilities|FlowControl|Delay 1.0)
  (bind _returnvalue (UserInterface|CreateWidget "/Game/Huds/HUD.HUD_C"))
  (UserInterface|Viewport|AddtoViewport _returnvalue 0))

(event Custom|Cam
  (bind _capsulecomponent (Variables|Collision|GetCapsuleComponent))
  (bind _returnvalue (Transformation|GetWorldLocation _capsulecomponent))
  (bind _z (Math|Vector|BreakVector _returnvalue))
  ;[1 1 1] Camera
  (if (<= (Variables|Default|GetCamera%20Level) _z)
    (Variables|/Script/Engine.SpringArmComponent|SetTargetOffset (Variables|Default|GetCamera%20Boom) (Math|Vector|MakeVector 0.0 0.0 (- (Variables|Default|GetCamera%20from%20ground) _z)))))

(event Custom|Death
  ;[1 1 1] Death & Respawn
  (Variables|Default|SetIs%20Dead true)
  (Utilities|FlowControl|Delay 0.1)
  (Input|DisableInput 0)
  (CameraFades|StartCameraFade (Game|GetPlayerCameraManager 0) 0.0 2.0 1.5 "(R=0.000000,G=0.000000,B=0.000000,A=1.000000)" false false)
  (Utilities|FlowControl|Delay 1.5)
  (Actor|DestroyActor)
  (CallFunction|SpawnNewChar))

(event EventTick
  (params (DeltaSeconds :type Float%20%28single-precision%29))
  ;[1 1 1] Every Tick
  (CallFunction|Cam)
  (if (Variables|Default|GetKill%20Z)
    (CallFunction|Death)
    (else
      (Variables|Default|SetKill%20Z (< (.Z (Math|Vector|BreakVector (Transformation|GetActorLocation))) -1e+03)))))

(event EventBeginPlay
  ;[1 1 1] On Start
  (CallFunction|SetHud)
  (bind _outactors (Actor|GetAllActorsOfClass 0))
  (Variables|Default|SetGlobal%20Var 0))

(event Input|ActionEvents|InputActionJump
  (params (Key :type Key%20Structure :default "AnyKey"))
  ;[1 1 1] Variable jump
  (:Pressed
    (if (Character|CanJump (Game|GetPlayerCharacter 0))
      (Character|Jump)))
  (:Released
    (Character|StopJumping)))

(event Input|AxisEvents|InputAxisMoveright
  (params (AxisValue :type Float%20%28single-precision%29))
  ;[1 1 1] Handle Movement
  (Pawn|Input|AddMovementInput "1.000000, 0, 0" AxisValue false)
  (CallFunction|UpdateAnim)
  ;[1 1 1] Handle Rotation
  (Math|Float|CompareFloat AxisValue 0.0
    (:>
      (Pawn|SetControlRotation (Pawn|GetController) (Math|Rotator|MakeRotator 0.0 0.0 0.0)))
    (:<
      (Pawn|SetControlRotation (Pawn|GetController) (Math|Rotator|MakeRotator 0.0 0.0 1.8e+02)))))

(event Input|KeyboardEvents|Q
  (params (Key :type Key%20Structure :default "AnyKey"))
  ;[1 1 1] Pause
  (:Pressed
    (Utilities|FlowControl|FlipFlop
      (:A
        (Game|SetGamePaused true)
        (Development|PrintString "Pause"))
      (:B
        (Game|SetGamePaused false)))))

(event Input|KeyboardEvents|Y
  (params (Key :type Key%20Structure :default "AnyKey"))
  ;[1 1 1] Death & Respawn
  (:Pressed
    (Variables|Default|SetIs%20Dead true)
    (Utilities|FlowControl|Delay 0.1)
    (Input|DisableInput 0)
    (CameraFades|StartCameraFade (Game|GetPlayerCameraManager 0) 0.0 2.0 1.5 "(R=0.000000,G=0.000000,B=0.000000,A=1.000000)" false false)
    (Utilities|FlowControl|Delay 1.5)
    (Actor|DestroyActor)
    (CallFunction|SpawnNewChar)))

(event Input|KeyboardEvents|J
  (params (Key :type Key%20Structure :default "AnyKey"))
  ;[1 1 1] Show Spawn Location
  (:Pressed
    (Development|PrintString (Utilities|String|ToString(Transform) (Variables|Default|GetCheckPoint)))))

(event Input|KeyboardEvents|U
  (params (Key :type Key%20Structure :default "AnyKey"))
  (:Pressed
    (bind _asglobal_var (Utilities|Casting|CastToGlobal_Var (Game|GetGameInstance)))
    (Utilities|FlowControl|FlipFlop
      (:A
        (bind _output_get (Variables|/Game/BluePrints/Global_Var.Global_Var_C|SetHas%20Item _asglobal_var true))
        (Development|PrintString (Utilities|String|ToString(Boolean) _output_get)))
      (:B
        (bind _output_get_2 (Variables|/Game/BluePrints/Global_Var.Global_Var_C|SetHas%20Item _asglobal_var false))
        (Development|PrintString (Utilities|String|ToString(Boolean) _output_get_2))))))

(fn ConstructionScript
  (Variables|Default|SetJumpMaxHoldTime (Variables|Default|GetMax%20jump%20hold))
  (Variables|Default|SetCheckPoint (Transformation|GetActorTransform))
  (Variables|Default|SetCamera%20from%20ground 1e+02))

(fn AnimationStateMachine
  (params (Is%20Falling :type Boolean) (Is%20Moving :type Boolean) (Is%20Dead :type Boolean))
  (Variables|Default|SetIs%20Falling Is%20Falling)
  (Variables|Default|SetIs%20Moving Is%20Moving)
  (Variables|Default|SetIs%20Dead Is%20Dead)
  (if (Variables|Default|GetIs%20Dead)
    (LocalVariables|SetAnimation%20State "NewEnumerator3")
    (elif (Variables|Default|GetIs%20Falling)
      (LocalVariables|SetAnimation%20State "NewEnumerator0")
      (elif (Variables|Default|GetIs%20Moving)
        (LocalVariables|SetAnimation%20State "NewEnumerator2")
        (else
          (LocalVariables|SetAnimation%20State "NewEnumerator1")))))
  (return (Utilities|Select :Index (LocalVariables|GetAnimation%20State) :NewEnumerator0 (Variables|Animations|GetFall) :NewEnumerator1 (Variables|Animations|GetIdle) :NewEnumerator2 (Variables|Animations|Getrun) :NewEnumerator3 (Variables|Animations|GetDead))))

(fn SpawnNewChar
  (bind _returnvalue (Game|SpawnActorfromClass "Char_Male_C" (Variables|Default|GetCheckPoint) "AdjustIfPossibleButAlwaysSpawn" 0 0))
  (Variables|Default|SetPlayer%20Pawn _returnvalue)
  (Pawn|Possess (Game|GetPlayerController 0) (Variables|Default|GetPlayer%20Pawn)))